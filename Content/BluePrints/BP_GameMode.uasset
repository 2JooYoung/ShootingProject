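; BP_GameMode is a game mode that starts a slime game and keeps a score.
; On BeginPlay it resets Score, prints a start message, and calls SpawnSlime in a loop to place ten BP_Slime actors.
; SpawnSlime drops each slime at a random X/Y position at a fixed height and prints its name.
; ScoreCount increments Score and prints the total on screen, but nothing in this Blueprint calls it.
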(event `self.ReceiveBeginPlay`
  (set `self.Score` 0)
  (`KismetSystemLibrary.PrintString` "GameStart!!!" true true (struct :`R` 1.0 :`G` 0.955964 :`A` 1.0))
  ; Spawn 10 Slimes
  (for _ (range 1 11)
    (`self.SpawnSlime`)
    (`KismetSystemLibrary.PrintString` "Hello")
    (`KismetSystemLibrary.PrintString` "Hello")))

(fn `ScoreCount`
  (bind _output_get (set `self.Score` (+ (`self.Score`) 1)))
  (`KismetSystemLibrary.PrintString` (`KismetTextLibrary.Conv_TextToString` (`|FormatText` "Score : {Score}" _output_get)) true true (struct :`R` 0.394246 :`G` 1.0 :`B` 0.220424 :`A` 1.0) 3.0))

(fn `SpawnSlime`
  (bind _returnvalue (`|SpawnActorFromClass` "/Game/BluePrints/BP_Slime.BP_Slime_C" (`KismetMathLibrary.MakeTransform` (`KismetMathLibrary.MakeVector` (`KismetMathLibrary.Conv_IntToDouble` (`KismetMathLibrary.RandomInteger` 1000)) (`KismetMathLibrary.Conv_IntToDouble` (`KismetMathLibrary.RandomInteger` 1000)) 200.0)) "Undefined" "MultiplyWithRoot" null null))
  (`KismetSystemLibrary.PrintString` (`KismetSystemLibrary.GetObjectName` _returnvalue)))

(fn `UserConstructionScript`)