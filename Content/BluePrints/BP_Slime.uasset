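; BP_Slime is a slime enemy with health, montage-driven attack, hit and death reactions, and a melee hit check.
; Attack plays the attack montage, while AttackPlayer separately sphere-traces forward and calls PlayerDamaged on a hit BP_Player.
; Damaged subtracts fixed health until death, then plays the death montage, unpossesses its controller and calls ScoreCount on BP_GameMode.
; Debug prints and trace drawing show spawn location, remaining health and attack range.
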(event `self.ReceiveBeginPlay`
  (set `self.IsDead` (`self.IsDead`))
  (set `self.Hp` (`self.MaxHp`))
  (`KismetSystemLibrary.PrintString` (`KismetStringLibrary.Conv_VectorToString` (`self.K2_GetActorLocation`)) true true (struct :`G` 0.66 :`B` 1.0 :`A` 1.0) 5.0))

(fn `Attack`
  (`self.PlayAnimMontage` "/Game/Animations/AM_SlimeAttack.AM_SlimeAttack"))

(fn `AttackPlayer`
  (bind _returnvalue (`self.K2_GetActorLocation`))
  (bind _outhit (`KismetSystemLibrary.SphereTraceSingle` :`Start` _returnvalue :`End` (+ _returnvalue (* (`self.GetActorForwardVector`) 200.0)) :`Radius` 100.0 :`TraceChannel` "TraceTypeQuery1" :`DrawDebugType` "ForDuration"))
  (if true
    (bind _asbp_player (cast `/Game/BluePrints/BP_Player` (`.HitActor` (`GameplayStatics.BreakHitResult` _outhit))))
    (`/Game/BluePrints/BP_Player.PlayerDamaged` _asbp_player)))

(fn `Damaged`
  (bind _returnvalue (`self.GetController`))
  (if (not (`self.IsDead`))
    (`self.PlayAnimMontage` "/Game/Animations/AM_SlimeDamaged.AM_SlimeDamaged")
    (set `self.Hp` (- (`self.Hp`) 3.0))
    (if (<= (`self.Hp`) 0.0)
      (set `self.Hp` 0.0)
      (set `self.IsDead` true))
    (`KismetSystemLibrary.PrintText` (`|FormatText` "Slime Hp : { Hp}" (`self.Hp`)) true true (struct :`R` 1.0 :`B` 0.773031 :`A` 1.0))
    (if (<= (`self.Hp`) 0.0)
      (`self.PlayAnimMontage` "/Game/Animations/AM_SlimeDead.AM_SlimeDead")
      (`/Engine/EditorBlueprintResources/StandardMacros.IsValid` _returnvalue
        (:`Is Valid`
          (`Controller.UnPossess` _returnvalue)
          (bind _asbp_game_mode (cast `/Game/BluePrints/BP_GameMode` (`GameplayStatics.GetGameMode`)))
          (`/Game/BluePrints/BP_GameMode.ScoreCount` _asbp_game_mode))))))

(fn `UserConstructionScript`)