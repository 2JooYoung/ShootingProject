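; Behavior tree service that supplies the player to an AI through the Player blackboard key.
; Its event, which takes the owner actor and delta seconds, runs a validity check and then writes BPPlayer to the key.
; The branch is hardwired to true, so the clearing path never runs and a 500-unit distance check to the owner sits unused.
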(event `CustomEvent`
  (params (OwnerActor :type "Actor Object Reference") (DeltaSeconds :type "Float (single-precision)"))
  (`/Engine/EditorBlueprintResources/StandardMacros.IsValid` null
    (:`Is Valid`
      (if true
        (`BTFunctionLibrary.SetBlackboardValueAsObject` (`self.Player`) (`self.BP_Player`))
        (else
          (`BTFunctionLibrary.SetBlackboardValueAsObject` (`self.Player`)))))))