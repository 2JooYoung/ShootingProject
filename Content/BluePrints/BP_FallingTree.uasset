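; BP_FallingTree is a tree actor that topples when Fall is called and can hurt the player on the way down.
; Fall sets IsFalling, which makes Tick play a Timeline that drives the actor's pitch until it finishes and clears the flag.
; Capsule hits during the fall call PlayerTreeDamaged on BP_Player, limited by a DoOnce that is never reset.
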(event `self.Capsule.OnComponentHit`
  (params (HitComponent :type "PrimitiveComponent Object Reference") (OtherActor :type "Actor Object Reference") (OtherComp :type "PrimitiveComponent Object Reference") (NormalImpulse :type "Vector Structure") (Hit :type "HitResult Structure (by ref)"))
  (if (`self.IsFalling`)
    (bind _asbp_player (cast `/Game/BluePrints/BP_Player` OtherActor))
    (`/Engine/EditorBlueprintResources/StandardMacros.DoOnce` false
      (:`Completed`
        (`/Game/BluePrints/BP_Player.PlayerTreeDamaged` _asbp_player)))))

(event `self.ReceiveTick`
  (params (DeltaSeconds :type "Float (single-precision)"))
  (if (`self.IsFalling`)
    (bind (_direction _pitch) (`Timeline|Timeline`)
      (:`Update`
        (`self.K2_SetActorRotation` (`KismetMathLibrary.MakeRotator` 0.0 _pitch)))
      (:`Finished`
        (set `self.IsFalling` false)))))

(fn `Fall`
  (set `self.IsFalling` true))

(fn `UserConstructionScript`)