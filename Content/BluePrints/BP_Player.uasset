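; BP_Player is the player pawn, handling shooting and a simple HP pool shown each tick as debug text.
; Fire plays a montage and line-traces from the deprojected screen center, calling Damaged on a hit BP_Slime or Fall on a BP_FallingTree.
; A second camera-forward trace runs but its result is unused.
; Separate functions subtract slime-sized or heavier tree damage and heal up to MaxHp, with no death check.
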(event `self.ReceiveBeginPlay`
  (set `self.Hp` (`self.MaxHp`)))

(event `self.ReceiveTick`
  (params (DeltaSeconds :type "Float (single-precision)"))
  (`KismetSystemLibrary.PrintString` (`KismetTextLibrary.Conv_TextToString` (`|FormatText` "PlayerHp : {hp} \n" (`self.Hp`))) true true (struct :`G` 0.66 :`B` 1.0 :`A` 1.0) 0.0))

(fn `Fire`
  (bind _returnvalue (`self.K2_GetActorLocation`))
  (bind (_returnvalue_x _returnvalue_y) (`KismetMathLibrary.BreakVector2D` (`WidgetLayoutLibrary.GetViewportSize`)))
  (bind (_worldposition _worlddirection) (`GameplayStatics.DeprojectScreenToWorld` (`GameplayStatics.GetPlayerController` 0) (`KismetMathLibrary.MakeVector2D` (/ _returnvalue_x 2.0) (/ _returnvalue_y 2.0))))
  (`self.PlayAnimMontage` "/Game/Animations/AM_Player.AM_Player")
  (bind _outhit (`KismetSystemLibrary.LineTraceSingle` _worldposition (+ _worldposition (* _worlddirection 5000.0)) "TraceTypeQuery1"))
  (`KismetSystemLibrary.LineTraceSingle` :`Start` _returnvalue :`End` (+ _returnvalue (* (`SceneComponent.GetForwardVector` (`self.Camera`)) 1000.0)) :`TraceChannel` "TraceTypeQuery1" :`TraceColor` (struct :`R` 1.0 :`G` 0.767609 :`A` 1.0) :`TraceHitColor` (struct :`R` 0.090273 :`B` 1.0 :`A` 1.0))
  (bind (_bblockinghit _binitialoverlap _time _distance _location _impactpoint _normal _impactnormal _physmat _hitactor) (`GameplayStatics.BreakHitResult` _outhit))
  (bind _asbp_slime (cast `/Game/BluePrints/BP_Slime` _hitactor)
    (:`then`
      (`/Game/BluePrints/BP_Slime.Damaged` _asbp_slime))
    (:`CastFailed`
      (bind _asbp_falling_tree (cast `/Game/BluePrints/BP_FallingTree` _hitactor))
      (`/Game/BluePrints/BP_FallingTree.Fall` _asbp_falling_tree))))

(fn `PlayerDamaged`
  (set `self.Hp` (- (`self.Hp`) 1.0)))

(fn `PlayerHpUp`
  (if (>= (`self.Hp`) (`self.MaxHp`))
    (set `self.Hp` (`self.MaxHp`))
    (else
      (set `self.Hp` (+ (`self.Hp`) 1.0)))))

(fn `PlayerTreeDamaged`
  (`KismetSystemLibrary.PrintString` "Hit By a Tree!" true true (struct :`R` 1.0 :`G` 0.159271 :`A` 1.0))
  (set `self.Hp` (- (`self.Hp`) 10.0)))

(fn `UserConstructionScript`)